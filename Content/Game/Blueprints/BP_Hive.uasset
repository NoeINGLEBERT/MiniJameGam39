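; BP_Hive is a spawner actor that populates the area around itself with a swarm of BP_MiGo actors at BeginPlay.
; A loop spawns about a hundred at random offsets around the hive, each given a random initial velocity and the hive's location.
; Roughly a quarter are randomly flagged as scouts, which draw their Speed from a faster range, assigned after the initial velocity is computed.
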(event `self.ReceiveBeginPlay`
  (for _ (range 101)
    (bind _returnvalue (`|SpawnActorFromClass` "/Game/Game/Blueprints/BP_MiGo.BP_MiGo_C" (`KismetMathLibrary.MakeTransform` (+ (`self.K2_GetActorLocation`) (* (`KismetMathLibrary.RandomUnitVector`) (`KismetMathLibrary.RandomFloatInRange` 200.0 2000.0)))) "Undefined" "MultiplyWithRoot" null null))
    (set `/Game/Game/Blueprints/BP_MiGo.Velocity` (* (`KismetMathLibrary.RandomUnitVector`) (`/Game/Game/Blueprints/BP_MiGo.Speed` _returnvalue) 2.0) _returnvalue)
    (set `/Game/Game/Blueprints/BP_MiGo.HiveLocation` (`self.K2_GetActorLocation`) _returnvalue)
    (bind _output_get (set `/Game/Game/Blueprints/BP_MiGo.IsScout` (> (`KismetMathLibrary.RandomFloat`) 0.75) _returnvalue))
    (set `/Game/Game/Blueprints/BP_MiGo.Speed` (`KismetMathLibrary.SelectFloat` (`KismetMathLibrary.RandomFloatInRange` 16666.666667 23333.333333) (`KismetMathLibrary.RandomFloatInRange` 12500.0 17500.0) _output_get) _returnvalue)))

(fn `UserConstructionScript`)
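; BP_MenuPlayer drives the main menu scene, showing the menu widget and mouse cursor and playing a world camera shake on BeginPlay.
; ToggleCredits uses a FlipFlop to switch between two fixed camera poses.
; One side fills the WBP_Text widgets in components D, B and N from the Text array, and the other clears them.
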(event `self.ReceiveBeginPlay`
  (bind _returnvalue (`|CreateWidget` "/Game/Game/Widgets/WBP_Menu.WBP_Menu_C"))
  (`UserWidget.AddToViewport` _returnvalue 0)
  (set `PlayerController.bShowMouseCursor` true (`GameplayStatics.GetPlayerController` 0))
  (`GameplayStatics.PlayWorldCameraShake` "/Game/Game/Blueprints/BP_MenuShake.BP_MenuShake_C" (`self.K2_GetActorLocation`) 10000.0 10000000.0))

(event `ToggleCredits`
  (bind _camera (`self.Camera`))
  (`/Engine/EditorBlueprintResources/StandardMacros.FlipFlop`
    (:`A`
      (for (_array_element _array_index) (`|MakeArray` (`self.D`) (`self.B`) (`self.N`))
        (bind _aswbp_text (cast `/Game/Game/Widgets/WBP_Text` (`WidgetComponent.GetWidget` _array_element)))
        (set `/Game/Game/Widgets/WBP_Text.Text` (`|GetArrayItem` (`self.Text`) _array_index) _aswbp_text))
      (`SceneComponent.K2_SetRelativeLocationAndRotation` _camera (-71.568939 5.0 134.322731) (struct :`Pitch` -27.408753) false false))
    (:`B`
      (for _array_element_2 (`|MakeArray` (`self.D`) (`self.B`) (`self.N`))
        (bind _aswbp_text_2 (cast `/Game/Game/Widgets/WBP_Text` (`WidgetComponent.GetWidget` _array_element_2)))
        (set `/Game/Game/Widgets/WBP_Text.Text` "" _aswbp_text_2))
      (`SceneComponent.K2_SetRelativeLocationAndRotation` _camera (-281.641777 164.943065 144.311061) (struct :`Pitch` -23.367821 :`Yaw` -38.883874) false false))))

(fn `UserConstructionScript`)
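; BP_Thunder is a lightning effect actor that flashes a plane mesh every few seconds.
; A randomly delayed loop fires Strike, whose timeline drives the plane material's "Y" parameter and a scaled "Emmiter" value.
; A separate looping timer eases the actor's pitch toward the look-at direction from the cached BP_GameMode's location to the actor, setting only that axis.
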(event `self.ReceiveBeginPlay`
  (bind _asbp_game_mode (cast `/Game/Game/Blueprints/BP_GameMode` (`GameplayStatics.GetGameMode`)))
  (set `self.As BP Game Mode` _asbp_game_mode)
  (`|ExecutionSequence`
    (:`then_0`
      (`KismetSystemLibrary.Delay` (`KismetMathLibrary.RandomFloatInRange` 4.0 5.0) :!label _label)
      (`self.Strike`)
      (goto _label))
    (:`then_1`
      (bind _returnvalue (`KismetSystemLibrary.K2_SetTimerDelegate` (delegate `Rotate`) 0.05 true))
      (set `self.Timer Handle` _returnvalue))))

(event `Rotate`
  (bind (_returnvalue_roll _returnvalue_pitch) (`KismetMathLibrary.BreakRotator` (`KismetMathLibrary.RInterpTo` (`self.K2_GetActorRotation`) (`KismetMathLibrary.FindLookAtRotation` (`self.K2_GetActorLocation` (`self.As BP Game Mode`)) (`self.K2_GetActorLocation`)) (`GameplayStatics.GetWorldDeltaSeconds`) 1.0)))
  (`self.K2_SetActorRotation` (`KismetMathLibrary.MakeRotator` 0.0 _returnvalue_pitch)))

(event `Strike`
  (bind _thunder_plane (`self.Thunder_Plane`))
  (bind (_direction _newtrack_0) (`Timeline|ThunderStrike`)
    (:`Update`
      (`MeshComponent.SetScalarParameterValueOnMaterials` _thunder_plane "Y" _newtrack_0)
      (`MeshComponent.SetScalarParameterValueOnMaterials` _thunder_plane "Emmiter" (* (+ _newtrack_0 1.0) 50.0)))))

(fn `UserConstructionScript`)
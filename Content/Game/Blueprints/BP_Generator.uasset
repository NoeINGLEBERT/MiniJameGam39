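; BP_Generator is a generator actor that plays a refill animation when given a jerrycan.
; Its Refill event plays a fill sound and attaches the jerrycan to the generator.
; A timeline lerps the can's relative transform between the Start and End component transforms, forcing unit scale each update, then destroys the can when finished.
; The file holds no fuel or power logic, only this presentation.
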(event `Refill`
  (params (Jerrycan :type "Actor Object Reference"))
  (`GameplayStatics.PlaySound2D` "/Game/Game/SoundDesign/SC_Fill.SC_Fill" 1.0 1.0 0.0 null null)
  (`self.K2_AttachToActor` Jerrycan self "None" "KeepRelative" "KeepRelative" "KeepRelative" true)
  (bind (_direction _alpha) (`Timeline|Timeline` :!via `PlayFromStart`)
    (:`Update`
      (`self.K2_SetActorRelativeTransform` Jerrycan (`KismetMathLibrary.TLerp` (`SceneComponent.GetRelativeTransform` (`self.Start`)) (`SceneComponent.GetRelativeTransform` (`self.End`)) _alpha) false false)
      (`self.SetActorScale3D` Jerrycan (1.0 1.0 1.0)))
    (:`Finished`
      (`self.K2_DestroyActor` Jerrycan))))

(fn `UserConstructionScript`)
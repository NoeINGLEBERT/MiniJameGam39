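; BP_MiGo is a flying swarm enemy that scouts for the player, returns to the hive when it spots them, then turns hunter.
; Tick steers by randomized velocity blending, repels it from BP_Tour towers and damages the player through BP_GameMode within hit range.
; MiGo relay screams through the GameMode, and non-scouts head toward any carrying a lower travelled-distance-to-player counter, spreading the player's location without pathfinding.
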(event `Hear`
  (params (Location :type "Vector Structure") (HiveCounter :type "Float (double-precision)") (PlayerCounter :type "Float (double-precision)"))
  (bind _gamemode (`self.GameMode`))
  (bind (_returnvalue_x _returnvalue_y) (`KismetMathLibrary.BreakVector` (`KismetMathLibrary.Normal` (- Location (`self.K2_GetActorLocation`)))))
  (bind (_returnvalue_x_2 _returnvalue_y_2 _returnvalue_z) (`KismetMathLibrary.BreakVector` (`KismetMathLibrary.Normal` (- (`self.K2_GetActorLocation` (`GameplayStatics.GetPlayerPawn` 0)) (`self.K2_GetActorLocation`)))))
  (if (< (`KismetMathLibrary.Vector_Distance` Location (`self.K2_GetActorLocation`)) (`self.ScreamRange`))
    (if (`self.IsScout`)
      _
      (elif (and (< PlayerCounter (`self.PlayerDistanceCounter`)) (< PlayerCounter 999999999.0))
        (set `self.IsSearching` false)
        (set `self.IsScout` false)
        (set `self.PlayerDistanceCounter` PlayerCounter)
        (set `self.TargetDir` (`KismetMathLibrary.Normal` (`KismetMathLibrary.MakeVector` _returnvalue_x _returnvalue_y _returnvalue_z)))
        (set `/Game/Game/Blueprints/BP_GameMode.AwokenMiGo` (+ (`/Game/Game/Blueprints/BP_GameMode.AwokenMiGo` _gamemode) (`GameplayStatics.GetWorldDeltaSeconds`)) _gamemode)))))

(event `self.ReceiveBeginPlay`
  (set `self.Player` (`GameplayStatics.GetPlayerPawn` 0))
  (`|ExecutionSequence`
    (:`then_0`
      (bind _asbp_game_mode (cast `/Game/Game/Blueprints/BP_GameMode` (`GameplayStatics.GetGameMode`)))
      (bind _output_get (set `self.GameMode` _asbp_game_mode))
      (add `/Game/Game/Blueprints/BP_GameMode.Scream` _output_get (delegate `Hear`)))
    (:`then_1`
      (`KismetSystemLibrary.Delay` (`KismetMathLibrary.RandomFloatInRange` 0.0 3.0))
      (`ActorComponent.Activate` (`self.SC_Buzzing`) false))
    (:`then_2`
      (bind _outactors (`GameplayStatics.GetAllActorsOfClass` "/Game/Game/Blueprints/BP_Tour.BP_Tour_C"))
      (for _array_element _outactors
        (`KismetArrayLibrary.Array_Add` (`self.TowerLocation`) (`self.K2_GetActorLocation` _array_element))))))

(event `self.ReceiveTick`
  (params (DeltaSeconds :type "Float (single-precision)"))
  (bind (_returnvalue_x _returnvalue_y _returnvalue_z) (`KismetMathLibrary.BreakVector` (`self.K2_GetActorLocation`)))
  (bind (_returnvalue_x_2 _returnvalue_y_2 _returnvalue_z_2) (`KismetMathLibrary.BreakVector` (`self.K2_GetActorLocation`)))
  (bind (_returnvalue_x_3 _returnvalue_y_3) (`KismetMathLibrary.BreakVector` (`self.K2_GetActorLocation`)))
  (bind _returnvalue (`self.K2_GetActorLocation`))
  (bind (_returnvalue_x_4 _returnvalue_y_4 _returnvalue_z_3) (`KismetMathLibrary.BreakVector` (`self.K2_GetActorLocation`)))
  (bind _returnvalue_2 (`self.K2_GetActorLocation`))
  (bind _screamrange (`self.ScreamRange`))
  (bind _velocity (`self.Velocity`))
  (bind (_hivelocation_x _hivelocation_y) (`KismetMathLibrary.BreakVector` (`self.HiveLocation`)))
  (bind _hivelocation (`self.HiveLocation`))
  (bind (_velocity_x _velocity_y _velocity_z) (`KismetMathLibrary.BreakVector` (`self.Velocity`)))
  (bind (_returnvalue_x_5 _returnvalue_y_5 _returnvalue_z_4) (`KismetMathLibrary.BreakVector` (`self.K2_GetActorLocation` (`GameplayStatics.GetPlayerPawn` 0))))
  (bind _returnvalue_3 (`self.K2_GetActorLocation` (`GameplayStatics.GetPlayerPawn` 0)))
  (bind _returnvalue_4 (* _velocity DeltaSeconds))
  (bind _returnvalue_5 (`KismetMathLibrary.Vector_Distance` (`KismetMathLibrary.MakeVector` _returnvalue_x_5 _returnvalue_y_5) (`KismetMathLibrary.MakeVector` _returnvalue_x _returnvalue_y)))
  (bind _returnvalue_6 (`KismetMathLibrary.VSize` _returnvalue_4))
  (bind _returnvalue_7 (`KismetMathLibrary.Normal` (- _hivelocation (`self.K2_GetActorLocation`))))
  (`|ExecutionSequence`
    (:`then_0`
      (set `self.Velocity` (`KismetMathLibrary.VLerp` (`self.Velocity`) (* (`KismetMathLibrary.RandomUnitVectorInConeInDegrees` (`KismetMathLibrary.VLerp` (`self.TargetDir`) (`KismetMathLibrary.Normal` (`self.Velocity`)) (`self.Reactivity`)) (`self.Randomness`)) (`self.Speed`)) (* DeltaSeconds (`self.SpeedReactivity`))))
      (`self.K2_SetActorLocationAndRotation` (+ (`self.K2_GetActorLocation`) _returnvalue_4) (`KismetMathLibrary.MakeRotFromXZ` _velocity (0.0 0.0 1.0)))
      (set `self.HiveDistanceCounter` (+ (`self.HiveDistanceCounter`) _returnvalue_6))
      (set `self.PlayerDistanceCounter` (+ (`self.PlayerDistanceCounter`) _returnvalue_6))
      (`SceneComponent.K2_SetWorldLocation` (`self.Plane`) (`KismetMathLibrary.MakeVector` _returnvalue_x_3 _returnvalue_y_3 125010.0) false false)
      (`|ExecutionSequence`
        (:`then_0`
          (if (< _returnvalue_z_2 0.0)
            (`self.K2_SetActorLocation` (`KismetMathLibrary.MakeVector` _returnvalue_x_2 _returnvalue_y_2 (* _returnvalue_z_2 -1.0)))
            (set `self.Velocity` (`KismetMathLibrary.MakeVector` _velocity_x _velocity_y (* _velocity_z -1.0)))))
        (:`then_1`
          (if (`self.IsSearching`)
            (set `self.TargetDir` (`KismetMathLibrary.SelectVector` (`KismetMathLibrary.Normal` (`KismetMathLibrary.VLerp` (`self.TargetDir`) (`KismetMathLibrary.Normal` (`KismetMathLibrary.VLerp` (`KismetMathLibrary.RandomUnitVectorInConeInDegrees` (`KismetMathLibrary.NegateVector` _returnvalue_7) 15.0) (`KismetMathLibrary.RandomUnitVectorInConeInDegrees` (- _returnvalue_3 _returnvalue) 15.0) (`KismetMathLibrary.FClamp` (* (`GameplayStatics.GetWorldDeltaSeconds`) (/ (* (`KismetMathLibrary.Vector_Distance` _hivelocation _returnvalue) (`KismetMathLibrary.Vector_Distance` _returnvalue_3 _returnvalue)) 10000000000.0))))) (* (`GameplayStatics.GetWorldDeltaSeconds`) 2.0))) _returnvalue_7 (`self.IsScout`)))))
        (:`then_2`
          (if (< _returnvalue_5 (`self.VisionRange`))
            (`self.PlayerSeen`)
            (if (< _returnvalue_5 (`self.HitRange`))
              (`/Engine/EditorBlueprintResources/StandardMacros.Gate` true :!label _label
                (:`Exit`
                  (`/Game/Game/Blueprints/BP_GameMode.Damage` (`self.GameMode`) (`self.K2_GetActorLocation`))
                  (goto _label :!via `Close`)))
              (else
                (goto _label :!via `Open`)))
            (else
              (goto _label :!via `Open`))))
        (:`then_3`
          (`KismetSystemLibrary.Delay` (`KismetMathLibrary.RandomFloatInRange` 0.2 0.3))
          (`/Game/Game/Blueprints/BP_GameMode.Scream` (`self.GameMode`) (`self.K2_GetActorLocation`) (+ (`self.HiveDistanceCounter`) _screamrange) (+ (`self.PlayerDistanceCounter`) _screamrange)))
        (:`then_4`
          (if (< (`KismetMathLibrary.Vector_Distance` (`KismetMathLibrary.MakeVector` _hivelocation_x _hivelocation_y) (`KismetMathLibrary.MakeVector` _returnvalue_x_4 _returnvalue_y_4)) (`self.VisionRange`))
            (if (and (`self.IsScout`) (not (`self.IsSearching`)))
              (set `self.IsScout` false)
              (set `self.TargetDir` (`KismetMathLibrary.NegateVector` (`self.TargetDir`)))
              (set `self.Randomness` 45.0)
              (set `self.Reactivity` 0.875)
              (set `self.Speed` (* (`self.Speed`) 0.5))
              (set `self.SpeedReactivity` 5.0))))))
    (:`then_1`
      (for _array_element (`self.TowerLocation`)
        (if (< (`KismetMathLibrary.Vector_Distance` (`KismetMathLibrary.MakeVector` (.x _returnvalue_2) (.y _returnvalue_2)) (`KismetMathLibrary.MakeVector` (.x _array_element) (.y _array_element))) 50000.0)
          (bind _returnvalue_8 (`KismetMathLibrary.Normal` (- _returnvalue_2 _array_element)))
          (set `self.TargetDir` _returnvalue_8)
          (set `self.Velocity` (* _returnvalue_8 (`KismetMathLibrary.VSize` (`self.Velocity`)))))))))

(event `PlayerSeen`
  (bind _isscout (`self.IsScout`))
  (if (and _isscout (`self.IsSearching`))
    (set `self.IsSearching` false)
    (`GameplayStatics.PlaySound2D` "/Game/Game/SoundDesign/SoundCue/SC_Scream.SC_Scream" 1.0 1.0 0.0 null null)
    (set `self.TargetDir` (- (`self.HiveLocation`) (`self.K2_GetActorLocation`)))
    (set `self.Randomness` 30.0)
    (set `self.Reactivity` 0.75)
    (set `self.Speed` (* (`self.Speed`) 1.5))
    (set `self.SpeedReactivity` 10.0)
    (set `self.PlayerDistanceCounter` (`KismetMathLibrary.Vector_Distance` (`self.K2_GetActorLocation` (`GameplayStatics.GetPlayerPawn` 0)) (`self.K2_GetActorLocation`)) :!label _label_2)
    (else
      (`|ExecutionSequence`
        (:`then_0`
          (if (== (`KismetMathLibrary.RandomIntegerInRange` 0 1000) 0)
            (`GameplayStatics.PlaySoundAtLocation` "/Game/Game/SoundDesign/SoundCue/SC_Scream.SC_Scream" (`self.K2_GetActorLocation`) (struct) 1.0 1.0 0.0 null null null null)))
        (:`then_1`
          (if (not _isscout)
            (set `self.TargetDir` (`KismetMathLibrary.Normal` (- (`self.K2_GetActorLocation` (`GameplayStatics.GetPlayerPawn` 0)) (`self.K2_GetActorLocation`))))
            (goto _label_2)
            (else
              (goto _label_2))))))))

(event `/Game/Game/Blueprints/BPI_Insect.Insect`
  (params (Center :type "Vector Structure"))
  (`KismetSystemLibrary.PrintString` "Hello")
  (set `self.TargetDir` (`KismetMathLibrary.Normal` (- (`self.K2_GetActorLocation`) Center)))
  (set `self.Velocity` (0.0 0.0 0.0)))

(fn `UserConstructionScript`)
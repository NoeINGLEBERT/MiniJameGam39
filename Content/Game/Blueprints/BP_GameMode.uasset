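; BP_GameMode is the game mode that handles damage to the player's BP_Plane and decides when it dies.
; It caches the player's plane on BeginPlay.
; Its Damage event increments the plane's hit counter, plays a hit sound and shakes the camera at the plane's camera position, leaving the Location input unused.
; Once the count passes a fixed threshold, it calls the plane's Death.
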(event `self.ReceiveBeginPlay`
  (bind _asbp_plane (cast `/Game/Game/Blueprints/BP_Plane` (`GameplayStatics.GetPlayerPawn` 0)))
  (set `self.Plane` _asbp_plane))

(event `Damage`
  (params (Location :type "Vector Structure"))
  (bind _plane (`self.Plane`))
  (bind _result (`/Engine/EditorBlueprintResources/StandardMacros.IncrementInt` (`/Game/Game/Blueprints/BP_Plane.Hit` _plane))
    (:`  `
      (`GameplayStatics.SpawnSound2D` "/Game/Game/SoundDesign/SC_Hit.SC_Hit" 1.0 1.0 0.0 null)
      (`GameplayStatics.PlayWorldCameraShake` "/Game/Game/Blueprints/BP_CameraShake.BP_CameraShake_C" (`SceneComponent.K2_GetComponentLocation` (`/Game/Game/Blueprints/BP_Plane.Camera` _plane)) 100.0 400.0)
      (if (> _result 20)
        (`/Game/Game/Blueprints/BP_Plane.Death` _plane)))))

(fn `UserConstructionScript`)